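; Follow camera for the chicken in a tile-based game, moving its spring arm forward each tick and easing sideways to the chicken's position on landing.
; Forward speed comes from a curve scaled by AdvanceSpeed, quadrupled when the chicken is ahead of the tile row found by a screen-centre line trace.
; Forward motion stops when the chicken dies; the too-far-behind check and killed handler take no action.
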(event Custom|OnChickenLanded
  (CallFunction|AlignHorizontalwithChicken))

(event Custom|OnChickenKilled)

(event EventBeginPlay
  (bind _chicken (Variables|Default|GetChicken))
  (Utilities|FlowControl|Sequence
    (:then_0
      (EventDispatchers|BindEventtoLanded _chicken (delegate Custom|OnChickenLanded)))
    (:then_1
      (EventDispatchers|BindEventtoKilled _chicken (delegate Custom|OnChickenKilled)))))

(event EventTick
  (params (DeltaSeconds :type Float%20%28single-precision%29))
  (bind _springarm (Variables|Default|GetSpringArm))
  (bind _relativelocation (Variables|/Script/Engine.SceneComponent|GetRelativeLocation _springarm))
  (Utilities|FlowControl|Sequence
    (:then_0
      ;[1 1 1] Update easing factor
      (Variables|Default|SetHorizontalMovementTime (Math|Float|Clamp(Float) (+ (Utilities|Time|GetWorldDeltaSeconds) (Variables|Default|GetHorizontalMovementTime)) 0.0 (Variables|Default|GetHorizontalEaseDelay))))
    (:then_1
      (CallFunction|UpdateTargetLocation 0.0)
      (Transformation|SetWorldLocation (Variables|Default|GetSpringArm) (+ (Math|Vector|MakeVector (.x _relativelocation) 0.0 (.z _relativelocation)) (Math|Vector|MakeVector (stale _deltax) (stale _deltay) 0.0)) false false))
    (:then_2
      (bind _deltax (CallFunction|GetForwardDelta DeltaSeconds))
      (bind _deltay (CallFunction|GetHorizontalDelta)))
    (:then_3
      (CallFunction|CheckChickenTooFar))))

(fn ConstructionScript)

(fn AlignHorizontalwithChicken
  (bind _chicken (Variables|Default|GetChicken))
  (Utilities|IsValid _chicken
    (:Is%20Valid
      (Utilities|FlowControl|Sequence
        (:then_0
          (Variables|Default|SetTargetPosition (Math|Vector|MakeVector (.x (Variables|Default|GetTargetPosition)) (.y (Transformation|GetActorLocation _chicken)) (.z (Variables|Default|GetTargetPosition)))))
        (:then_1
          (Variables|Default|SetHorizontalMovementTime 0.0))
        (:then_2
          (Variables|Default|SetHorizontalSource (.y (Transformation|GetWorldLocation (Variables|Default|GetSpringArm)))))))))

(fn GetForwardDelta
  (params (Delta%20Seconds :type Float%20%28single-precision%29))
  (bind _advancespeed (Variables|Default|GetAdvanceSpeed))
  (bind _springarm (Variables|Default|GetSpringArm))
  (bind _targetposition (Variables|Default|GetTargetPosition))
  (bind _advancespeed_2 (Variables|Default|GetAdvanceSpeed))
  (bind _forwardmotioncurve (Variables|Default|GetForwardMotionCurve))
  (bind _chicken (Variables|Default|GetChicken))
  (bind _returnvalue (Transformation|GetRelativeTransform _springarm))
  (bind _returnvalue_2 (- (.x _targetposition) (.x (.location _returnvalue))))
  (bind _returnvalue_3 (/ _returnvalue_2 _advancespeed_2))
  (bind _returnvalue_4 (Math|Curves|GetFloatValue _forwardmotioncurve _returnvalue_3))
  (bind _returnvalue_5 (* _returnvalue_4 _advancespeed))
  (bind _returnvalue_6 (* _returnvalue_5 Delta%20Seconds))
  (Utilities|IsValid _chicken
    (:Is%20Valid
      (if (not (Variables|/Game/Blueprints/BP_Chicken.BP_Chicken_C|GetDead _chicken))
        (bind _camlaneindex (CallFunction|GetLookatIndex))
        (if (> (- (Variables|/Game/Blueprints/BP_Chicken.BP_Chicken_C|GetYLocation _chicken) _camlaneindex) 0)
          (return (* 4.0 _returnvalue_6))
          (else
            (return _returnvalue_6)))
        (else
          _)))
    (:Is%20Not%20Valid
      _))
  ;[1 1 1] Apply one last delta update as though chicken were alive and enable camera lag so camera slows to a stop
  (return 0.0))

(fn GetHorizontalDelta
  (return (Math|Interpolation|Ease "EaseOut" (/ (Variables|Default|GetHorizontalMovementTime) (Variables|Default|GetHorizontalEaseDelay)) (Variables|Default|GetHorizontalSource) (.y (Variables|Default|GetTargetPosition)) 1.0)))

(fn UpdateTargetLocation
  (params (Delta%20Seconds :type Float%20%28single-precision%29))
  (bind _chicken (Variables|Default|GetChicken))
  (Utilities|IsValid _chicken
    (:Is%20Valid
      (Variables|Default|SetTargetPosition (Math|Vector|MakeVector (+ (* Delta%20Seconds (Variables|Default|GetAdvanceSpeed)) (.x (Variables|Default|GetTargetPosition))) (.y (Variables|Default|GetTargetPosition)) (.z (Transformation|GetActorLocation _chicken)))))
    (:Is%20Not%20Valid
      (Variables|Default|SetTargetPosition (Math|Vector|MakeVector (+ (* Delta%20Seconds (Variables|Default|GetAdvanceSpeed)) (.x (Variables|Default|GetTargetPosition))) (.y (Variables|Default|GetTargetPosition)) (.z (Variables|Default|GetTargetPosition)))))))

(fn CheckChickenTooFar
  (bind _chicken (Variables|Default|GetChicken))
  (Utilities|IsValid _chicken
    (:Is%20Valid
      (bind _camlaneindex (CallFunction|GetLookatIndex))
      ;[1 1 1] If chicken too far behind camera, kill it
      (if (> (- _camlaneindex (Variables|/Game/Blueprints/BP_Chicken.BP_Chicken_C|GetYLocation _chicken)) 3)
        _))))

(fn GetLookatIndex
  (bind _returnvalue (Viewport|GetViewportSize))
  (bind _camera (Variables|Default|GetCamera))
  (bind _returnvalue_2 (Transformation|GetWorldLocation _camera))
  (Utilities|IsValid (Variables|Default|GetChicken)
    (:Is%20Valid
      (bind (_outhit _returnvalue_3) (Collision|LineTraceByChannel _returnvalue_2 (+ (* (.WorldDirection (Class|GameplayStatics|DeprojectScreentoWorld (Game|GetPlayerController 0) (Math|Vector2D|MakeVector2D (* (.x _returnvalue) 0.5) (* (.y _returnvalue) 0.5)))) 1e+03) _returnvalue_2) "TraceTypeQuery3" false 0 "None"))
      (if _returnvalue_3
        (bind _y (CallFunction|GetTileCoordsfromMapSpacePosition (.Location (Collision|BreakHitResult _outhit)) (Variables|/Game/Blueprints/GM_TopDown.GM_TopDown_C|GetTileSize (Variables|Default|GetGameMode))))
        (return _y)))))