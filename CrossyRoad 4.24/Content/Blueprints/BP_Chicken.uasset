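; Player chicken for a Crossy Road-style game, hopping between tiles and lanes.
; Jump checks lane passability, box-traces water lanes for landing actors, then launches the physics mesh on a computed ballistic impulse while Tick rotates it.
; Ground hits snap position and rotation to the grid and restore input; crouching squashes the mesh.
; Leaving bounds detaches the view via a stationary camera; Kill currently only disables input, bypassing its death effects.
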(event OnComponentHit(ChickenMesh)
  (params (HitComponent :type Primitive%20Component%20Object%20Reference) (OtherActor :type Actor%20Object%20Reference) (OtherComp :type Primitive%20Component%20Object%20Reference) (NormalImpulse :type Vector :default "0, 0, 0") (Hit :type Hit%20Result%20Structure%20%28by%20ref%29))
  ;[1 1 1] Trigger On Landed
  (if (and (Components|ComponentHasTag OtherComp "Ground") (Variables|Default|GetIsAirborne))
    (Variables|Default|SetIsAirborne false)
    (CallFunction|OnLanded)))

(event Custom|OnLanded
  (bind _gamemode (Variables|Default|GetGameMode))
  (bind _chickenmesh (Variables|Default|GetChickenMesh))
  ;[1 1 1] On Landed Event
  (Utilities|IsValid self
    (:Is%20Valid
      (Utilities|FlowControl|Sequence
        (:then_0
          (if (Variables|Default|GetIsOnGrid)
            (bind _alignedworldposition (CallFunction|GetMapAlignedPosition (Transformation|GetActorLocation) _gamemode))
            (Transformation|SetActorLocation _alignedworldposition false true))
          (CallFunction|UpdateSelfLocationCoords))
        (:then_1
          (Class|PrimitiveComponent|SetAllPhysicsLinearVelocity _chickenmesh "0, 0, 0" false)
          (Class|PrimitiveComponent|SetAllPhysicsAngularVelocityinRadians _chickenmesh (Math|Vector|MakeVector 0.0 0.0 0.0) false))
        (:then_2
          (bind (_alignedrotation _compassdir) (CallFunction|GetMapAlignedRotation (Transformation|GetWorldRotation _chickenmesh) _gamemode))
          (Transformation|SetActorRotation _alignedrotation true)
          (Variables|Default|SetFacingDirection _compassdir))
        (:then_3
          (Input|EnableInput (Game|GetPlayerController 0) 0))
        (:then_4
          (Default|CallLanded))
        (:then_5
          (Variables|Default|SetCrouchFactor 0.33) ; Add a little bounce on landing
        )))))

(event EventBeginPlay
  ;[1 1 1] Setup
  (Utilities|FlowControl|Sequence
    (:then_0
      (bind _asgm_top_down (Utilities|Casting|CastToGM_TopDown (Game|GetGameMode)))
      (Variables|Default|SetGameMode _asgm_top_down))
    (:then_1
      (Variables|Default|SetForwardImpulse (/ (.x (Variables|/Game/Blueprints/GM_TopDown.GM_TopDown_C|GetTileSize (Variables|Default|GetGameMode))) (Variables|Default|GetJumpTime))))
    (:then_2
      (CallFunction|UpdateSelfLocationCoords))))

(event EventTick
  (params (DeltaSeconds :type Float%20%28single-precision%29))
  (bind _gamemode (Variables|Default|GetGameMode))
  (bind _camera (Variables|/Game/Blueprints/GM_TopDown.GM_TopDown_C|GetCamera _gamemode))
  (if (not (Variables|Default|GetDead))
    (Utilities|FlowControl|Sequence
      (:then_0
        (CallFunction|UpdateCrouch DeltaSeconds))
      (:then_1
        ;[1 1 1] Handle chicken mid-air rotation
        (if (Variables|Default|GetIsAirborne)
          (bind _output_get (Variables|Default|SetTimeInAir (+ DeltaSeconds (Variables|Default|GetTimeInAir))))
          (Transformation|SetActorRotation (Math|Rotator|Lerp(Rotator) (Variables|Default|GetStartRotation) (Variables|Default|GetTargetRotation) (Math|Float|Min(Float) (/ _output_get (Variables|Default|GetTimeToRotate)) 1.0) true) true)))
      (:then_2
        (bind _outofbounds (CallFunction|IsOutOfBounds))
        (if _outofbounds
          (Utilities|FlowControl|Sequence
            (:then_0
              (bind _returnvalue (Game|SpawnActorfromClass "/Game/Blueprints/BP_StationaryCamera.BP_StationaryCamera_C" (Transformation|GetActorTransform _camera) "AlwaysSpawn" 0 0))
              (Transformation|SetRelativeTransform (Variables|/Game/Blueprints/BP_StationaryCamera.BP_StationaryCamera_C|GetSpringArm _returnvalue) (Transformation|GetRelativeTransform (Variables|/Game/Blueprints/BP_Camera.BP_Camera_C|GetSpringArm _camera)) false true))
            (:then_1
              (Input|DisableInput (Game|GetPlayerController 0) 0))
            (:then_3
              (Audio|PlaySound2D 0 1.0 1.0 0.0 0 0))))))))

(fn ConstructionScript)

(fn Jump
  (params (Direction :type E_Compass%20Enum :default "NewEnumerator0"))
  (bind _returnvalue (Transformation|GetActorLocation))
  (bind _jumpsounds (Variables|Default|GetJumpSounds))
  (if (not (Variables|Default|GetIsAirborne))
    (Utilities|FlowControl|Sequence
      (:then_0
        (bind (_targetlocation _isvalidjump _isongrid) (CallFunction|SweepforLandingLocation Direction))
        (if (or _isvalidjump (not _isongrid))
          (Utilities|FlowControl|Sequence
            (:then_0
              (Variables|Default|SetIsOnGrid _isongrid))
            (:then_1
              (Variables|Default|SetIsAirborne true))
            (:then_2
              (Input|DisableInput (Game|GetPlayerController 0) 0)
              (Variables|Default|SetIsCrouching false))
            (:then_3
              (bind _outrotation (CallFunction|CompassDirectiontoRotation Direction))
              (Variables|Default|SetStartRotation (Math|Rotator|MakeRotator 0.0 0.0 (.yaw (Transformation|GetActorRotation))))
              (Variables|Default|SetTargetRotation (Math|Rotator|MakeRotator 0.0 0.0 (.yaw _outrotation)))
              (Variables|Default|SetTimeInAir 0.0))
            (:then_4
              (bind _impulseforcevelocity (CallFunction|CalculateTrajectoryImpulse (Transformation|GetWorldLocation (Variables|Default|GetChickenMesh)) _targetlocation))
              (Class|PrimitiveComponent|SetAllPhysicsLinearVelocity (Variables|Default|GetChickenMesh) "0, 0, 0" false)
              (Physics|AddImpulse (Variables|Default|GetChickenMesh) _impulseforcevelocity "None" true)
              (Default|CallJumped))
            (:then_5
              ;[1 1 1] Play the hop sound most of the time, with some random bocks in there
              (if (Math|Random|RandomBoolwithWeight 0.55)
                (Audio|PlaySoundatLocation 0 _returnvalue "0, 0, 0" 1.0 1.0 0.0 0 0 0)
                (else
                  (Audio|PlaySoundatLocation (Utilities|Array|Get(acopy) _jumpsounds (Math|Random|RandomIntegerinRange 0 (Utilities|Array|Length _jumpsounds))) _returnvalue "0, 0, 0" 1.0 1.0 0.0 0 0 0))))))))))

(fn UpdateSelfLocationCoords
  (bind (_x _y) (CallFunction|GetTileCoordsfromMapSpacePosition (.location (Math|Transform|MakeRelativeTransform (Math|Transform|MakeTransform (.location (Transformation|GetActorTransform))) (Transformation|GetActorTransform (Variables|/Game/Blueprints/GM_TopDown.GM_TopDown_C|GetMapRoot (Variables|Default|GetGameMode))))) (Variables|/Game/Blueprints/GM_TopDown.GM_TopDown_C|GetTileSize (Variables|Default|GetGameMode))))
  (Utilities|FlowControl|Sequence
    (:then_0
      (Variables|Default|SetXLocation _x))
    (:then_1
      (Variables|Default|SetYLocation _y))))

(fn CalculateTrajectoryImpulse
  (params (StartLocationWorld :type Vector) (TargetLocationWorld :type Vector))
  (bind _returnvalue (Math|Vector|Distance2D(Vector) (Math|Vector|MakeVector (.x StartLocationWorld) (.y StartLocationWorld) 0.0) (Math|Vector|MakeVector (.x TargetLocationWorld) (.y TargetLocationWorld) 0.0)))
  (bind _returnvalue_2 (Math|Vector|MakeVector (.x TargetLocationWorld) (.y TargetLocationWorld) 0.0))
  (bind _returnvalue_3 (Math|Vector|MakeVector (.x StartLocationWorld) (.y StartLocationWorld) 0.0))
  (bind _jumptime (Variables|Default|GetJumpTime))
  (bind _returnvalue_4 (- _returnvalue_2 _returnvalue_3))
  (bind _returnvalue_5 (/ _returnvalue _jumptime))
  (bind _returnvalue_6 (Math|Vector|Normalize _returnvalue_4))
  (bind _returnvalue_7 (* _returnvalue_6 _returnvalue_5))
  (return (Math|Vector|MakeVector (.x _returnvalue_7) (.y _returnvalue_7) (/ (- (- (.z TargetLocationWorld) (.z StartLocationWorld)) (* (* (* _jumptime _jumptime) (Variables|Default|GetGravity)) 0.5)) _jumptime))))

(fn Kill
  (params (Death%20Type :type Byte :default 0))
  (bind _returnvalue (Transformation|GetActorTransform))
  (bind _deathsoundshit (Variables|Default|GetDeathSoundsHit))
  (bind _returnvalue_2 (+ (.location _returnvalue) "0, 0,50.000000"))
  (if (not (Variables|Default|GetDead))
    (if true
      (Input|DisableInput (Game|GetPlayerController 0) 0)
      (else
        (Utilities|FlowControl|Sequence
          (:then_0
            (Variables|Default|SetDead true)
            (Rendering|SetVisibility (Variables|Default|GetChickenMesh) false true))
          (:then_1
            (switch Utilities|FlowControl|Switch|Switchon Death%20Type
              (:NewEnumerator0
                (Effects|SpawnEmitteratLocation "/Game/Blueprints/PS_Feathers.PS_Feathers" (.location _returnvalue) (.rotation _returnvalue) (.scale _returnvalue))
                (Audio|SpawnSoundatLocation (Utilities|Array|Get(acopy) _deathsoundshit (Math|Random|RandomIntegerinRange 0 (Utilities|Array|Length _deathsoundshit))) (.location _returnvalue) "0, 0, 0" 1.0 1.0 0.0 0 0))
              (:NewEnumerator1
                (bind _groundposition (CallFunction|GetGroundUnderChicken :!label _label)))
              (:NewEnumerator2
                (goto _label))
              (:NewEnumerator3
                (Effects|SpawnEmitteratLocation 0 _returnvalue_2 (.rotation _returnvalue) (.scale _returnvalue))
                (Audio|SpawnSoundatLocation 0 (.location _returnvalue) "0, 0, 0" 1.0 1.0 0.0 0 0)
                (Audio|SpawnSoundatLocation 0 _returnvalue_2 "0, 0, 0" 1.0 1.0 0.0 0 0))))
          (:then_2)
          (:then_3
            (Default|CallKilled)
            (Actor|DestroyActor)))))))

(fn SweepforLandingLocation
  (params (Direction :type E_Compass%20Enum :default "NewEnumerator0"))
  (bind _returnvalue (Transformation|GetActorLocation))
  (bind _gamemode (Variables|Default|GetGameMode))
  (bind _gamemode_2 (Variables|Default|GetGameMode))
  (bind _chickenmesh (Variables|Default|GetChickenMesh))
  (bind _returnvalue_2 (Transformation|GetWorldLocation _chickenmesh))
  (bind _tilesize (Variables|/Game/Blueprints/GM_TopDown.GM_TopDown_C|GetTileSize _gamemode_2))
  (bind _tilesize_2 (Variables|/Game/Blueprints/GM_TopDown.GM_TopDown_C|GetTileSize _gamemode))
  (CallFunction|UpdateSelfLocationCoords)
  (bind (_relativexcoord _relativeycoord) (CallFunction|CompassDirectiontoRelativeTileCoord Direction))
  (bind _outrotation (CallFunction|CompassDirectiontoRotation Direction))
  (LocalVariables|SetChickenForwardTileUnaligned (+ (Math|Vector|MakeVector (.x _returnvalue) (.y _returnvalue) 0.0) (Math|Vector|RotateVector (Math|Vector|MakeVector (.x _tilesize) 0.0 0.0) _outrotation)))
  ;[1 1 1] Jump is allowed?
  (bind (_lane _found) (Default|GetLanebyIndex (Variables|/Game/Blueprints/GM_TopDown.GM_TopDown_C|GetMapRoot (Variables|Default|GetGameMode)) (+ _relativeycoord (Variables|Default|GetYLocation))))
  (if _found
    (if (Utilities|Array|Get(acopy) (Variables|/Game/Blueprints/Map/BP_LaneBase.BP_LaneBase_C|GetLanePassability _lane) (+ _relativexcoord (Variables|Default|GetXLocation)))
      ;[1 1 1] Grid jump or physics jump?
      (if (== (.Spawner (Utilities|Struct|BreakBPS_Spawner (Variables|/Game/Blueprints/Map/BP_LaneBase.BP_LaneBase_C|GetSpawnerInfo _lane))) "/Game/Blueprints/Map/BP_WaterLane.BP_WaterLane_C")
        (bind (_outhits _returnvalue_3) (Class|KismetSystemLibrary|BoxTraceMulti (LocalVariables|GetChickenForwardTileUnaligned) (+ (* (Math|Vector|GetForwardVector _outrotation) 0.01) (LocalVariables|GetChickenForwardTileUnaligned)) (Math|Vector|MakeVector (* (.y _tilesize) 0.33) (* (* (.x _tilesize) 0.5) 1.2) 32.0) "0, 0, 0" "TraceTypeQuery4" true 0 "None" true))
        ;[1 1 1] Find closest thing to land on, if there are multiple possibilities. We consider velocity here
        (if _returnvalue_3
          (for _array_element _outhits
            (bind (_haslandingpoints _nearestpredictedlandingpoint) (CallFunction|GetNearestLandingMarker (.HitActor (Collision|BreakHitResult _array_element))))
            (if _haslandingpoints
              (LocalVariables|SetLandingActorPredictedLocation _nearestpredictedlandingpoint)
              (LocalVariables|SetLandingActorRef (.HitActor (Collision|BreakHitResult _array_element)))))
          (Utilities|IsValid (LocalVariables|GetLandingActorRef)
            (:Is%20Valid
              (return (LocalVariables|GetLandingActorPredictedLocation) true false))
            (:Is%20Not%20Valid
              _)))
        ;[1 1 1] Aim for a grid coordinate, even though we know nothing's there
        (bind _alignedworldposition (CallFunction|GetMapAlignedPosition (LocalVariables|GetChickenForwardTileUnaligned) (Variables|Default|GetGameMode)))
        (return (Math|Vector|MakeVector (.x _alignedworldposition) (.y _alignedworldposition) 1e+01) false false)
        (else
          ;[1 1 1] Target is a tile coordinate
          (return (+ (Math|Vector|MakeVector (.x _returnvalue_2) (.y _returnvalue_2) 0.0) (Math|Vector|MakeVector (* _relativeycoord (.x _tilesize_2)) (* _relativexcoord (.y _tilesize_2)) (.LaneZHeight (Utilities|Struct|BreakBPS_Spawner (Variables|/Game/Blueprints/Map/BP_LaneBase.BP_LaneBase_C|GetSpawnerInfo _lane))))) true true)))
      (else
        _)))
  (return "0, 0, 0" false (Variables|Default|GetIsOnGrid)))

(fn GetNearestLandingMarker
  (params (Target :type Actor%20Object%20Reference))
  (if (not (Utilities|DoesObjectImplementInterface Target 0))
    (return false "0, 0, 0")))

(fn UpdateCrouch
  (params (DeltaTime :type Float%20%28single-precision%29))
  (bind _returnvalue (Math|Float|MakeLiteralFloat 0.75))
  (if (Variables|Default|GetIsCrouching)
    (Variables|Default|SetCrouchFactor (Math|Float|Min(Float) (+ (* (Math|Float|MakeLiteralFloat 2.0) DeltaTime) (Variables|Default|GetCrouchFactor)) 1.0))
    (else
      ;[1 1 1] 'Uncrouch' over time
      (bind _output_get (Variables|Default|SetCrouchFactor (Math|Float|Max(Float) (- (Variables|Default|GetCrouchFactor) (* (Math|Float|MakeLiteralFloat 3.0) DeltaTime)) 0.0)))))
  (Transformation|SetRelativeScale3D (Variables|Default|GetChickenMesh) (Math|Vector|MakeVector (+ (* (* (Math|Float|MakeLiteralFloat 1.0) _output_get) 0.1) 1.0) (+ (* (* (Math|Float|MakeLiteralFloat 1.0) _output_get) 0.1) 1.0) (+ (* (- 1.0 (Variables|Default|GetCrouchFactor)) (- 1.0 _returnvalue)) _returnvalue))))

(fn Crouch
  (if (not (Variables|Default|GetIsAirborne))
    (Variables|Default|SetIsCrouching true)))

(fn StopCrouching
  (Variables|Default|SetIsCrouching false))

(fn GetGroundUnderChicken
  (bind _returnvalue (Transformation|GetActorLocation))
  (bind (_outhit _returnvalue_2) (Collision|LineTraceByChannel (Math|Vector|MakeVector (.x _returnvalue) (.y _returnvalue) 1e+02) (Math|Vector|MakeVector (.x _returnvalue) (.y _returnvalue) -1e+02) "TraceTypeQuery3" false 0 "None"))
  (if _returnvalue_2
    (return (.ImpactPoint (Collision|BreakHitResult _outhit)))
    (else
      (return (Transformation|GetActorLocation)))))

(fn IsOutOfBounds
  (bind _gamemode (Variables|Default|GetGameMode))
  (bind _tilesize (Variables|/Game/Blueprints/GM_TopDown.GM_TopDown_C|GetTileSize _gamemode))
  (bind _playabletilesinlane (Variables|/Game/Blueprints/GM_TopDown.GM_TopDown_C|GetPlayableTilesInLane _gamemode))
  (bind _returnvalue (+ _playabletilesinlane 2))
  (bind _returnvalue_2 (* _returnvalue (.y _tilesize)))
  (bind _returnvalue_3 (* _returnvalue_2 0.5))
  (return (not (Math|Float|InRange(Float) (.y (Transformation|GetActorLocation)) (* _returnvalue_3 -1.0) _returnvalue_3))))