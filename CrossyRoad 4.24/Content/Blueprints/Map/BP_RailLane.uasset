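; Rail lane for the tile-based map, with a crossing sign that flashes and plays a sound when triggered.
; BeginPlay assigns rail tile meshes for passable and impassable ground, runs the parent setup, hides the lit sign parts and positions the sign from lane width and tile size.
; TriggerSign starts a short countdown, and UpdateAnimation re-arms itself by timer to alternate sign meshes and lights, then restores the off state.
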(event EventBeginPlay
  (bind _railsignposition (Variables|Default|GetRailSignPosition))
  (bind _gamemode (Variables|Default|GetGameMode))
  (bind _returnvalue (Transformation|GetRelativeTransform _railsignposition))
  (bind _tilesize (Variables|/Game/Blueprints/GM_TopDown.GM_TopDown_C|GetTileSize _gamemode))
  (Utilities|FlowControl|Sequence
    (:then_0
      (Variables|Default|SetPassableGroundTile (Variables|Default|GetISM_Rail))
      (Variables|Default|SetImpassableGroundTile (Variables|Default|GetISM_Rail_Dark))
      (Utilities|FlowControl|Sequence
        (:then_0
          (Rendering|SetVisibility (Variables|Default|GetSM_SignOn1) false false))
        (:then_1
          (Rendering|SetVisibility (Variables|Default|GetSM_SignOn2) false false))
        (:then_2
          (Rendering|SetVisibility (Variables|Default|GetLeftLight) false false))
        (:then_3
          (Rendering|SetVisibility (Variables|Default|GetRightLight) false false))))
    (:then_1
      (|CallParentFunction))
    (:then_2
      (CallFunction|GetObstacleSpawnerWorldTransform (Variables|Default|GetGameMode) self))
    (:then_4
      ;[1 1 1] Center sign, then align with left boundary
      (Transformation|SetRelativeLocation _railsignposition (Math|Vector|MakeVector (.x (.location _returnvalue)) (+ (* (* (Variables|/Game/Blueprints/GM_TopDown.GM_TopDown_C|GetMaxTilesInLane _gamemode) (.y _tilesize)) 0.5) (* 0.5 (.y _tilesize))) (.z (.location _returnvalue))) false false))))

(fn ConstructionScript
  (|CallParentFunction))

(fn TriggerSign
  (Utilities|FlowControl|Sequence
    (:then_0
      (Rendering|SetVisibility (Variables|Default|GetSM_SignOff) false false))
    (:then_1
      (Rendering|SetVisibility (Variables|Default|GetSM_SignOn1) true false)
      (Rendering|SetVisibility (Variables|Default|GetLeftLight) true false)
      (Rendering|SetVisibility (Variables|Default|GetRightLight) false false))
    (:then_2
      (Rendering|SetVisibility (Variables|Default|GetSM_SignOn2) false false))
    (:then_3
      (Variables|Default|SetTimeLeftToStayOn 1.5))
    (:then_4
      (Audio|SpawnSoundAttached 0 (Variables|Default|GetRailSignPosition) "None" "0, 0, 0" "0, 0, 0" "KeepRelativeOffset" false 1.0 1.0 0.0 0 0))
    (:then_5
      (Utilities|Time|SetTimerbyFunctionName 0 "UpdateAnimation" (Variables|Default|GetSignFrameDuration)))))

(fn UpdateAnimation
  (bind _output_get (Variables|Default|SetTimeLeftToStayOn (Math|Float|Max(Float) (- (Variables|Default|GetTimeLeftToStayOn) (Variables|Default|GetSignFrameDuration)) 0.0)))
  (if (<= _output_get 0.0)
    (Utilities|FlowControl|Sequence
      (:then_0
        (Rendering|SetVisibility (Variables|Default|GetSM_SignOff) true false))
      (:then_1
        (Rendering|SetVisibility (Variables|Default|GetSM_SignOn1) false false))
      (:then_2
        (Rendering|SetVisibility (Variables|Default|GetSM_SignOn2) false false))
      (:then_3
        (Rendering|SetVisibility (Variables|Default|GetLeftLight) false false)
        (Rendering|SetVisibility (Variables|Default|GetRightLight) false false)))
    (else
      (Utilities|FlowControl|Sequence
        (:then_0
          (Rendering|ToggleVisibility (Variables|Default|GetSM_SignOn1) false)
          (Rendering|ToggleVisibility (Variables|Default|GetSM_SignOn2) false))
        (:then_1
          (Rendering|ToggleVisibility (Variables|Default|GetLeftLight) false)
          (Rendering|ToggleVisibility (Variables|Default|GetRightLight) false))
        (:then_2
          (Utilities|Time|SetTimerbyFunctionName 0 "UpdateAnimation" (Variables|Default|GetSignFrameDuration)))))))