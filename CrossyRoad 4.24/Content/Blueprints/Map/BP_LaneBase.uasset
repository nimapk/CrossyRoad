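; BP_LaneBase is a base lane actor that builds one row of ground tiles for a tile-based, top-down game.
; SpawnLane clears and refills passable and impassable instanced meshes, classifying each tile by the GameMode's playable zone and lane size.
; It records passability per index for GetPassable, which returns false out of range.
; Empty OnTileSpawned and OnLaneFinishedSpawning hooks allow extension, while SpawnCoinsMaybe is an empty stub.
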(event EventBeginPlay
  (bind _asgm_top_down (Utilities|Casting|CastToGM_TopDown (Game|GetGameMode)))
  (Variables|Default|SetGameMode _asgm_top_down))

(fn ConstructionScript)

(fn SpawnLane
  (bind _gamemode (Variables|Default|GetGameMode))
  (Utilities|FlowControl|Sequence
    (:then_0
      (Utilities|Array|Clear (Variables|Default|GetLanePassability))
      (Components|InstancedStaticMesh|ClearInstances (Variables|Default|GetPassableGroundTile))
      (Components|InstancedStaticMesh|ClearInstances (Variables|Default|GetImpassableGroundTile)))
    (:then_1
      (for _index (range 0 (- (Variables|/Game/Blueprints/GM_TopDown.GM_TopDown_C|GetMaxTilesInLane _gamemode) 1))
        (bind _iswithinplayablezone (CallFunction|TileIsinPlayableZone _gamemode _index))
        (bind _localtransform (CallFunction|GetTileTransformRelative _gamemode _index))
        (if _iswithinplayablezone
          (Components|InstancedStaticMesh|AddInstance (Variables|Default|GetPassableGroundTile) _localtransform)
          (else
            (Components|InstancedStaticMesh|AddInstance (Variables|Default|GetImpassableGroundTile) _localtransform)))
        (bind _returnvalue (Utilities|Array|Add (Variables|Default|GetLanePassability) _iswithinplayablezone))
        (CallFunction|OnTileSpawned _returnvalue _iswithinplayablezone)))
    (:then_2
      (CallFunction|OnLaneFinishedSpawning))))

(fn OnTileSpawned
  (params (Index :type Integer) (IsPassable :type Boolean))
  (return))

(fn OnLaneFinishedSpawning)

(fn GetPassable
  (params (Index :type Integer))
  (if (Math|Integer|InRange(Integer) Index 0 (Utilities|Array|Length (Variables|Default|GetLanePassability)) true false)
    (return (Utilities|Array|Get(acopy) (Variables|Default|GetLanePassability) Index))
    (else
      (return (Class|KismetSystemLibrary|MakeLiteralBool false)))))

(fn SpawnCoinsMaybe)