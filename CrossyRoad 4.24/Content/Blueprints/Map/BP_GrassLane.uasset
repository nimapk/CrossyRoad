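; Grass lane Blueprint for a tile-based lane map, setting grass ground tiles and scattering obstacles over them.
; As tiles spawn, impassable ones get blocking tree instances.
; After the first few lanes, passable tiles randomly gain instanced trees or rocks, up to a per-lane cap, and update lane passability.
; Once such a later lane finishes spawning, it may spawn coins.
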(event EventBeginPlay
  (Utilities|FlowControl|Sequence
    (:then_0
      (|CallParentFunction))
    (:then_1
      (Variables|Default|SetPassableGroundTile (Variables|Default|GetGroundGrass_Passable)))
    (:then_2
      (Variables|Default|SetImpassableGroundTile (Variables|Default|GetGroundGrass_Impassable)))))

(event EventOnLaneFinishedSpawning
  (if (> (Variables|/Game/Blueprints/GM_TopDown.GM_TopDown_C|GetLanesSpawned (Variables|Default|GetGameMode)) 8)
    (CallFunction|SpawnCoinsMaybe)))

(event EventOnTileSpawned
  (params (Index :type Integer) (IsPassable :type Boolean))
  (if IsPassable
    (if (and (> (Variables|/Game/Blueprints/GM_TopDown.GM_TopDown_C|GetLanesSpawned (Variables|Default|GetGameMode)) 8) (and (Math|Random|RandomBoolwithWeight 0.2) (<= (Variables|Default|GetObstacleCount) 4)))
      (Utilities|Array|SetArrayElem (Variables|Default|GetLanePassability) Index false)
      (bind _localtransform (CallFunction|GetTileTransformRelative (Variables|Default|GetGameMode) Index))
      (Math|Integer|IncrementInt (Variables|Default|GetObstacleCount)
        (:%20%20
          (switch int (Math|Random|RandomIntegerinRange 0 1)
            (:Default
              (Components|InstancedStaticMesh|AddInstance (Variables|Default|GetISM_Tree2) _localtransform :!label _label))
            (:0
              (goto _label))
            (:1
              (Components|InstancedStaticMesh|AddInstance (Variables|Default|GetISM_Rock1) _localtransform))))))
    (else
      (bind _localtransform_2 (CallFunction|GetTileTransformRelative (Variables|Default|GetGameMode) Index))
      (Components|InstancedStaticMesh|AddInstance (Variables|Default|GetBlockingTree) _localtransform_2))))

(fn ConstructionScript
  (|CallParentFunction))