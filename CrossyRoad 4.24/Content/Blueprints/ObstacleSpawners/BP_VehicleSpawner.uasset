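; BP_VehicleSpawner is an obstacle spawner that repeatedly spawns BP_Vehicle actors at its own transform.
; On BeginPlay it picks one random speed for all its vehicles and caches the GM_TopDown game mode.
; A non-looping timer re-arms itself with a new random delay after each spawn.
; Each vehicle attaches to the spawner and gets a lifespan of the game mode's travel distance divided by speed.
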(event Custom|SpawnVehicle_Event
  (Utilities|Time|ClearandInvalidateTimerbyHandle (stale _returnvalue))
  (CallFunction|Spawn)
  (bind _returnvalue (Utilities|Time|SetTimerbyEvent (delegate Custom|SpawnVehicle_Event) (Math|Random|RandomFloatinRange (Variables|Default|GetMinSpawnDelay) (Variables|Default|GetMaxSpawnDelay)))) ; no loop intended
)

(event EventBeginPlay
  (Utilities|FlowControl|Sequence
    (:then_0
      (Variables|Default|SetSpeed (Math|Random|RandomFloatinRange (Variables|Default|GetMinSpeed) (Variables|Default|GetMaxSpeed)))
      (bind _asgm_top_down (Utilities|Casting|CastToGM_TopDown (Game|GetGameMode)))
      (Variables|Default|SetGameMode _asgm_top_down))
    (:then_1
      (bind _travel_distance (CallFunction|GetVehicleTravelDistance (Variables|Default|GetGameMode)))
      (Variables|Default|SetTravelDistance _travel_distance))
    (:then_3
      (bind _returnvalue (Utilities|Time|SetTimerbyEvent (delegate Custom|SpawnVehicle_Event) (Math|Random|RandomFloatinRange (Variables|Default|GetMinSpawnDelay) (Variables|Default|GetMaxSpawnDelay)))) ; no loop intended
    )))

(fn ConstructionScript)

(fn Spawn
  (bind _gamemode (Variables|Default|GetGameMode))
  (bind _speed (Variables|Default|GetSpeed))
  (Utilities|FlowControl|Sequence
    (:then_0
      (bind _travel_distance (CallFunction|GetVehicleTravelDistance _gamemode)))
    (:then_1
      (bind _returnvalue (Game|SpawnActorfromClass "/Game/Blueprints/ObstacleSpawners/BP_Vehicle.BP_Vehicle_C" (Transformation|GetActorTransform) "AlwaysSpawn" 0 _speed _gamemode 0))
      (if (Utilities|IsValid _returnvalue)
        (Actor|SetLifeSpan _returnvalue (/ _travel_distance _speed))
        (Transformation|AttachActorToActor _returnvalue self "None" "KeepWorld" "KeepWorld" "KeepWorld" true)))))